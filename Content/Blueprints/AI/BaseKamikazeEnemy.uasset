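; Base kamikaze enemy that blows itself up to damage the player when it attacks.
; An attack, guarded to start only once, flashes the explosive barrel's material, changes walk speed and waits out the attack cooldown as a fuse.
; It then damages the player only if inside the explosion range, prints a debug message and destroys itself.
; Chasing is allowed while the enemy is chasing and not incapacitated.
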(event Custom|WaitBeforeExploding
  (Rendering|Material|SetScalarParameterValueonMaterials (Variables|Default|GetExplosiveBarrel) "FLashing" 1.0)
  (Variables|/Script/Engine.CharacterMovementComponent|SetMaxWalkSpeed (Variables|Character|GetCharacterMovement) 1.5e+02)
  (Utilities|FlowControl|Delay (Variables|Default|GetAttackCooldown))
  (if (Collision|IsOverlappingActor (Variables|Default|GetExplosionRange) (Game|Player|GetPlayerPawn 0) :!class /Script/Engine.PrimitiveComponent)
    (Game|Damage|ApplyDamage (Game|Player|GetPlayerPawn 0) (Variables|Default|GetBaseDamage) (AI|GetAIController self) (Components|GetOwner (Variables|Default|GetWeapon)))
    (Development|PrintString "PLAYER WAS IN EXPLOSION RANGE, OUCH" true true "(R=0.000000,G=0.660000,B=1.000000,A=1.000000)" 5.0)
    (else
      (Development|PrintString "PLAYER WAS NOT IN EXPLOSION RANGE :((((" true true "(R=0.000000,G=0.660000,B=1.000000,A=1.000000)" 5.0)))
  (Actor|DestroyActor))

(fn ConstructionScript
  (|CallParentFunction))

(fn AttackPlayer
  (if (Variables|Default|GetIsAttacking)
    (return)
    (else
      (Variables|Default|SetIsAttacking true)
      (CallFunction|WaitBeforeExploding))))

(fn CanChasePlayer
  (return (and (Variables|Default|GetIsChasing) (not (CallFunction|IsIncapacitated)))))

(fn TriggerAttackAnim
  (CallFunction|AttackPlayer))