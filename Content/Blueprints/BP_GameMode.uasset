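; BP_GameMode is a game mode Blueprint that checks whether the player has won by clearing enemy spawners.
; CheckVictoryStatus loops over all EnemySpawner actors, overwriting the win flag with each IsSpawnerCleared result, so only the last spawner decides the outcome.
; On a win, it casts player 0's HUD to TopdownHUD and calls OnVictory.
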(fn ConstructionScript)

(fn CheckVictoryStatus
  (LocalVariables|SetShouldWinGame false)
  (bind _outactors (Actor|GetAllActorsOfClass "/Game/Blueprints/Spawners/EnemySpawner.EnemySpawner_C"))
  (for _array_element _outactors
    (LocalVariables|SetShouldWinGame (Default|IsSpawnerCleared _array_element)))
  (if (LocalVariables|GetShouldWinGame)
    (bind _astopdown_hud (Utilities|Casting|CastToTopdownHUD (HUD|GetHUD (Game|GetPlayerController 0))))
    (Default|OnVictory _astopdown_hud)))