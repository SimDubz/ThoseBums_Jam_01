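; Enemy spawner that spawns up to a set number of enemies and notifies the game mode when all are killed.
; SpawnEnemy places the chosen class at a random navigable point around EnemySpawnerActor, raised slightly, then starts a cooldown that re-triggers spawning until the cap is reached.
; Each enemy's OnDestroyed increments the slain count; once it equals the maximum, BP_GameMode checks victory status.
; No event in this graph makes the first spawn call.
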(event Custom|SpawnEnemy_Event
  ;[1 1 1] Spawn enemy event
  (if (CallFunction|CanSpawnAnotherEnemy)
    (bind _randomlocation (Class|NavigationSystemV1|GetRandomLocationinNavigableRadius (.location (Transformation|GetWorldTransform (Variables|Default|GetEnemySpawnerActor))) 2e+03 0 0))
    (bind _returnvalue (Game|SpawnActorfromClass (Variables|Default|GetEnemyTypeToSpawn) (Math|Transform|MakeTransform (+ _randomlocation "0, 0,100.000000") "0, 0, 0" "1,1,1") "AdjustIfPossibleButAlwaysSpawn" 0 0))
    (CallFunction|SpawnCooldownEvent)
    (Math|Integer|IncrementInt (Variables|Default|GetSpawnedEnemiesQTS)
      (:%20%20
        (Game|BindEventtoOnDestroyed _returnvalue (delegate Custom|OnEnemyKilled))))))

(event Custom|OnEnemyKilled
  (params (DestroyedActor :type Actor%20Object%20Reference))
  ;[1 1 1] Spawn enemy event
  (Math|Integer|IncrementInt (Variables|Default|GetSlainedEnemiesQTS)
    (:%20%20
      (if (CallFunction|IsSpawnerCleared)
        (bind _asbp_game_mode (Utilities|Casting|CastToBP_GameMode (Game|GetGameMode)))
        (Default|CheckVictoryStatus _asbp_game_mode)))))

(event Custom|SpawnCooldown_Event
  ;[1 1 1] Spawn cooldown event
  (Variables|Default|SetIsInCooldown true)
  (Utilities|FlowControl|Delay (Variables|Default|GetSpawnCooldown))
  (Variables|Default|SetIsInCooldown false)
  (if (CallFunction|CanSpawnAnotherEnemy)
    (CallFunction|SpawnEnemyEvent)))

(fn ConstructionScript)

(fn CanSpawnAnotherEnemy
  (return (and (< (Variables|Default|GetSpawnedEnemiesQTS) (Variables|Default|GetMaxEnemies)) (not (Variables|Default|GetIsInCooldown)))))

(fn IsSpawnerCleared
  (return (== (Variables|Default|GetSlainedEnemiesQTS) (Variables|Default|GetMaxEnemies))))